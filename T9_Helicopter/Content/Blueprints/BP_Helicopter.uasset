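; Player-controlled helicopter that moves vertically within clamped bounds and explodes when it hits an obstacle.
; MoveUp input drives the frame-rate-scaled vertical offset, while the MoveForward horizontal logic is left unwired.
; Tick spins the Scene component by a fixed step each frame.
; Overlaps ignore coins; actors whose first tag is Block trigger explosion effects and sound, the OnDead dispatcher, then self-destruction.
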(event `self.ReceiveBeginPlay`)

(event `self.ReceiveActorBeginOverlap`
  (params (OtherActor :type "Actor Object Reference"))
  (bind (_returnvalue_location _returnvalue_rotation) (`KismetMathLibrary.BreakTransform` (`self.GetTransform`)))
  (cast `/Game/Blueprints/BP_Coin` OtherActor
    (:`CastFailed`
      (if (== (`|GetArrayItem` (`Actor.Tags` OtherActor)) "Block")
        (`|SpawnActorFromClass` "/Game/Blueprints/BP_ExplosionParticle.BP_ExplosionParticle_C" (`KismetMathLibrary.MakeTransform` _returnvalue_location _returnvalue_rotation (5.0 5.0 5.0)) "AlwaysSpawn" "OverrideRootScale" null null)
        (`GameplayStatics.PlaySoundAtLocation` "/Game/Sounds/explosion.explosion" (`self.K2_GetActorLocation`) (struct) 1.0 1.0 0.0 null null null)
        (`self.OnDead`)
        (`self.K2_DestroyActor`)))))

(event `self.ReceiveTick`
  (params (DeltaSeconds :type "Float (single-precision)"))
  (`SceneComponent.K2_AddLocalRotation` (`self.Scene`) (struct :`Yaw` 5.0) false false))

(event `InputAxis|MoveUp`
  (params (AxisValue :type "Float (single-precision)"))
  (bind (_returnvalue_x _returnvalue_y _returnvalue_z) (`KismetMathLibrary.BreakVector` (`self.K2_GetActorLocation`)))
  (`self.K2_AddActorWorldOffset` (`KismetMathLibrary.MakeVector` 0.0 0.0 (* AxisValue (`self.MoveSpeed`) (`GameplayStatics.GetWorldDeltaSeconds`))))
  (`self.K2_SetActorLocation` (`KismetMathLibrary.MakeVector` _returnvalue_x _returnvalue_y (`KismetMathLibrary.FClamp` _returnvalue_z -2000.0 2000.0))))

(event `InputAxis|MoveForward`
  (params (AxisValue :type "Float (single-precision)")))

(fn `UserConstructionScript`)