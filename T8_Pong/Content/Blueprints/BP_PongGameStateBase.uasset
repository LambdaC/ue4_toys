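; Game state Blueprint for a Pong game that keeps the left and right scores.
; On BeginPlay it finds the first BP_Ball in the level and binds to its BallOutOfBound event.
; When that event fires, a "LeftWall" first tag on the trigger wall gives the right side a point, any other gives the left side one.
; The ball is then re-initialized through InitBall.
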(event `self.ReceiveBeginPlay`
  (`|ExecutionSequence`
    (:`then_0`
      (bind _outactors (`GameplayStatics.GetAllActorsOfClass` "/Game/Blueprints/BP_Ball.BP_Ball_C"))
      (set `self.Ball` (`|GetArrayItem` _outactors)))
    (:`then_1`
      (add `/Game/Blueprints/BP_Ball.BallOutOfBound` (`self.Ball`) (delegate `BallOutOfBound_事件_0`)))))

(event `BallOutOfBound_事件_0`
  (params (TriggerWall :type "/Game/Blueprints/BP_TriggerWall Object Reference"))
  (if (== (`|GetArrayItem` (`Actor.Tags` TriggerWall)) "LeftWall")
    (`/Engine/EditorBlueprintResources/StandardMacros.IncrementInt` (`self.RightScore`)
      (:`  `
        _))
    (else
      (`/Engine/EditorBlueprintResources/StandardMacros.IncrementInt` (`self.LeftScore`)
        (:`  `
          _))))
  (`/Game/Blueprints/BP_Ball.InitBall` (`self.Ball`)))

(fn `UserConstructionScript`)