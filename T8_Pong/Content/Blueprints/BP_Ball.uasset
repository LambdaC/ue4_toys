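; BP_Ball is a ball actor that moves in a straight line until it overlaps another actor.
; The construction script picks a random horizontal Direction in the positive X/Y quadrant.
; While IsMoving is set, Tick applies Direction as an unswept local offset to the static mesh, without delta-time scaling.
; On overlap it re-sets its current location and clears IsMoving.
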(event `self.ReceiveActorBeginOverlap`
  (params (OtherActor :type "Actor Object Reference"))
  (`self.K2_SetActorLocation` (`self.K2_GetActorLocation`))
  (set `self.IsMoving` false))

(event `self.ReceiveTick`
  (params (DeltaSeconds :type "Float (single-precision)"))
  (if (`self.IsMoving`)
    (`SceneComponent.K2_AddLocalOffset` (`self.StaticMeshComponent`) (`self.Direction`) false false)))

(fn `UserConstructionScript`
  (bind _returnvalue (`KismetMathLibrary.RandomFloat`))
  (set `self.Direction` (`KismetMathLibrary.MakeVector` (* _returnvalue 20.0) (* (- 1.0 _returnvalue) 20.0))))