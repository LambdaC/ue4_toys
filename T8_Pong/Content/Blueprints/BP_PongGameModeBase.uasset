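; Game mode for a Pong game that sets up the HUD and runs the countdown before the ball starts moving.
; BeginPlay adds the HUD widget to the viewport and caches the first BP_Ball found in the level.
; OnBallReady resets the countdown and starts a looping one-second timer on CountDown, which sets the ball's IsMoving flag and clears the timer when time runs out.
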(event `self.ReceiveBeginPlay`
  (`|ExecutionSequence`
    (:`then_0`
      (bind _returnvalue (`|CreateWidget` "/Game/Blueprints/BP_HUD.BP_HUD_C"))
      (`UserWidget.AddToViewport` _returnvalue 0))
    (:`then_1`
      (bind _outactors (`GameplayStatics.GetAllActorsOfClass` "/Game/Blueprints/BP_Ball.BP_Ball_C"))
      (set `self.Ball` (`|GetArrayItem` _outactors)))))

(event `OnBallReady`
  (set `self.CountDownSeconds` (`self.MaxCountDownSeconds`))
  (`KismetSystemLibrary.K2_SetTimer` null "CountDown" 1.0 true))

(event `CountDown`
  (bind _result (`/Engine/EditorBlueprintResources/StandardMacros.DecrementInt` (`self.CountDownSeconds`))
    (:`  `
      (if (<= _result 0)
        (set `/Game/Blueprints/BP_Ball.IsMoving` true (`self.Ball`))
        (`KismetSystemLibrary.K2_ClearTimer` null "CountDown")))))

(fn `UserConstructionScript`)